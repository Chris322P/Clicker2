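; Game mode that persists money and a test bool and relays inventory changes to the player's inventory widget.
; BeginPlay loads the save slot or creates one, and EndPlay writes it back.
; After a successful load and short delay, it caches the controller's InventoryWidget and fills it with 16 debug items from test arrays.
; AddItem and RemoveItem forward to that widget; AddItem retains disconnected free-slot search logic.
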(event `self.ReceiveEndPlay`
  (params (EndPlayReason :type "EEndPlayReason Enum" :default "Destroyed"))
  (`self.SaveGame_`))

(event `self.ReceiveBeginPlay`
  (bind _returnvalue (`KismetTextLibrary.Conv_StringToText` (`KismetStringLibrary.Concat_StrStr` "ITEM " (`KismetStringLibrary.Conv_IntToString` (`self.TEST_VAL`)))))
  (bind _returnvalue_2 (`GameplayStatics.DoesSaveGameExist` (`self.SaveGame`)))
  (if _returnvalue_2
    (`self.LoadGame`)
    (`KismetSystemLibrary.PrintText` (`KismetTextLibrary.Conv_StringToText` (`KismetStringLibrary.Concat_StrStr` "Money: " (`self.GetMoney`))) true true (struct :`G` 0.66 :`B` 1.0 :`A` 1.0) 5.0)
    (`KismetSystemLibrary.PrintText` "LOADED")
    (`KismetSystemLibrary.Delay` 0.2)
    (bind _asplayer_controller_chris_bp (cast `/Game/Chris/PlayerControllerChrisBP` (`GameplayStatics.GetPlayerController` 0)))
    (set `self.inventroyWidget` (`/Game/Chris/PlayerControllerChrisBP.inventoryWidget` _asplayer_controller_chris_bp))
    (for _index (range 16)
      (bind _output (`|GetArrayItem` (`self.TEST_RND`) _index))
      (`KismetArrayLibrary.Array_Add` (`/Game/Chris/Interface/Inventory.Inventory_Items` (`self.inventroyWidget`)) (make `InventoryItem` 0 _returnvalue "Item" 0 _output (`|GetArrayItem` (`self.TEST_THUMB`) _index)))
      (set `self.TEST_VAL` (+ (`self.TEST_VAL`) 1))
      (`KismetSystemLibrary.PrintString` (`KismetStringLibrary.Concat_StrStr` "SLOT: " (`KismetStringLibrary.Conv_IntToString` _output) " ITEM: " (`KismetTextLibrary.Conv_TextToString` _returnvalue))))
    (else
      (`self.SaveGame_`))))

(fn `AddItem`
  (params (Item :type "InventoryItem Structure"))
  (locals (TMP_INVSLOTS :type "Array of Integer"))
  (`/Game/Chris/Interface/Inventory.addItem` (`self.inventroyWidget`) Item))

(fn `LoadGame`
  (bind _returnvalue (`GameplayStatics.LoadGameFromSlot` (`self.SaveGame`)))
  (bind _assave_game_bp (cast `/Game/Chris/SaveGameBP` _returnvalue))
  (bind _output_get (set `self.SaveGameReference` _assave_game_bp))
  (set `self.Bool1_GM` (`/Game/Chris/SaveGameBP.bool1` _output_get))
  (`self.SetMoney` (`/Game/Chris/SaveGameBP.money` _output_get)))

(fn `RemoveItem`
  (params (itemSlot :type Integer))
  (locals (itemSlotToRemove :type Integer))
  (`/Game/Chris/Interface/Inventory.removeItemAtSlot` (`self.inventroyWidget`) itemSlot))

(fn `SaveGame_`
  (bind _savegamereference (`self.SaveGameReference`))
  (`/Engine/EditorBlueprintResources/StandardMacros.IsValid` (`self.SaveGameReference`)
    (:`Is Valid`
      (set `/Game/Chris/SaveGameBP.bool1` (`self.Bool1_GM`) _savegamereference)
      (set `/Game/Chris/SaveGameBP.money` (`self.GetMoney`) _savegamereference))
    (:`Is Not Valid`
      (bind _returnvalue (`GameplayStatics.CreateSaveGameObject` "/Game/Chris/SaveGameBP.SaveGameBP_C"))
      (bind _output_get (set `self.SaveGameReference` _returnvalue))
      (set `self.Bool1_GM` (`/Game/Chris/SaveGameBP.bool1` _output_get))
      (`self.SetMoney` (`/Game/Chris/SaveGameBP.money` _output_get))))
  (`GameplayStatics.SaveGameToSlot` (`self.SaveGameReference`) (`self.SaveGame`)))

(fn `UserConstructionScript`)