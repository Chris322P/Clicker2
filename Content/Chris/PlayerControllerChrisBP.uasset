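; Player controller Blueprint that manages the game's screen widgets and shows the mouse cursor.
; ChangeMAP clears current widgets, creates the MAIN or KAMPF screen, then re-adds the HUD_INFO overlay through AddHUD.
; The Inventory input toggles a freshly created inventory widget, tracked by InventoryOpen and removed on close.
; BeginPlay opens the MAIN screen but also creates a second HUD_INFO, replacing the stored reference without removing the first.
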(event `InputAction|Inventory`
  (params (Key :type "Key Structure"))
  (:`Pressed`
    (if (`self.inventoryOpen`)
      (`self.closeInventory`)
      (else
        (bind _returnvalue (`|CreateWidget` "/Game/Chris/Inventory.Inventory_C" null "/Game/Chris/test_test.test_test"))
        (bind _output_get (set `self.inventoryWidget` _returnvalue))
        (`UserWidget.AddToViewport` _output_get 0)
        (set `self.inventoryOpen` true)))))

(event `self.ReceiveBeginPlay`
  (set `self.bShowMouseCursor` true)
  (`self.ChangeMAP` "NewEnumerator0")
  (bind _returnvalue (`|CreateWidget` "/Game/Chris/HUD_INFO.HUD_INFO_C"))
  (set `self.mainHUD` _returnvalue)
  (`UserWidget.AddToViewport` _returnvalue 0))

(event `self.ReceiveTick`
  (params (DeltaSeconds :type "Float (single-precision)")))

(fn `addHUD`
  (bind _returnvalue (`|CreateWidget` "/Game/Chris/HUD_INFO.HUD_INFO_C"))
  (bind _output_get (set `self.mainHUD` _returnvalue))
  (`UserWidget.AddToViewport` _output_get 0))

(fn `ChangeMAP`
  (params (Map :type "/Game/Chris/MAPS Enum" :default "NewEnumerator0"))
  (bind _mainhud (`self.mainHUD`))
  (bind _inventorywidget (`self.inventoryWidget`))
  (bind _curmap (`self.curMAP`))
  (`/Engine/EditorBlueprintResources/StandardMacros.IsValid` _inventorywidget
    (:`Is Valid`
      (`Widget.RemoveFromParent` _inventorywidget))
    (:`Is Not Valid`
      _))
  (`/Engine/EditorBlueprintResources/StandardMacros.IsValid` _mainhud
    (:`Is Valid`
      (`Widget.RemoveFromParent` _mainhud))
    (:`Is Not Valid`
      _))
  (`/Engine/EditorBlueprintResources/StandardMacros.IsValid` _curmap
    (:`Is Valid`
      (`Widget.RemoveFromParent` _curmap))
    (:`Is Not Valid`
      _))
  (bind _output_get (set `self.Maps` Map))
  (switch `/Game/Chris/MAPS` _output_get
    (:`NewEnumerator0`
      (bind _returnvalue (`|CreateWidget` "/Game/Chris/HUD_MAIN.HUD_MAIN_C"))
      (bind _output_get_2 (set `self.curMAP` _returnvalue))
      (`UserWidget.AddToViewport` _output_get_2 0))
    (:`NewEnumerator1`
      (bind _returnvalue_2 (`|CreateWidget` "/Game/Chris/HUD_KAMPF.HUD_KAMPF_C"))
      (bind _output_get_3 (set `self.curMAP` _returnvalue_2))
      (`UserWidget.AddToViewport` _output_get_3 0)))
  (`self.addHUD`)
  (set `self.inventoryOpen` false))

(fn `closeInventory`
  (`Widget.RemoveFromParent` (`self.inventoryWidget`))
  (set `self.inventoryOpen` false))

(fn `UserConstructionScript`)